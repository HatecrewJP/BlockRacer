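; Test car pawn that handles Enhanced Input actions for pausing the game and switching camera views.
; Pause toggles a newly created BlockCollector pause menu along with game pause, input mode and mouse cursor; closing also removes the menu's tracked sub-widgets.
; A FlipFlop on the camera action alternates between the third-person and second-person cameras, activating third-person on the first press.
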(event `EnhancedInput|/Game/Blueprints/Input/Driving/PauseGameBR`
  (params (ActionValue :type Boolean) (ElapsedSeconds :type "Float (double-precision)") (TriggeredSeconds :type "Float (double-precision)") (InputAction :type "InputAction Object Reference" :default "/Game/Blueprints/Input/Driving/PauseGameBR.PauseGameBR"))
  (bind _returnvalue (`GameplayStatics.GetPlayerController` 0))
  (bind _returnvalue_2 (`GameplayStatics.GetPlayerController` 0))
  (bind _pausemenuwidget (`self.PauseMenuWidget`))
  (:`Started`
    ;[1 1 1] Check if menu is open
    (if (not (`self.IsMenuOpen`))
      ;[1 1 1] Open Menu
      (set `self.IsMenuOpen` true)
      (bind _returnvalue_3 (`|CreateWidget` "/Game/Blueprints/UI/PauseMenu/BlockCollectorPauseMenuWidgetBR.BlockCollectorPauseMenuWidgetBR_C" _returnvalue_2))
      (bind _output_get (set `self.PauseMenuWidget` _returnvalue_3))
      (`UserWidget.AddToViewport` _output_get 0)
      (`UserWidget.AddToViewport` _returnvalue_3 0)
      (`WidgetBlueprintLibrary.SetInputMode_GameAndUIEx` _returnvalue_2 (`self.PauseMenuWidget`))
      (set `PlayerController.bShowMouseCursor` true (`GameplayStatics.GetPlayerController` 0))
      (`GameplayStatics.SetGamePaused` true)
      (else
        ;[1 1 1] Close Menu
        (set `self.IsMenuOpen` false)
        ;;[1 1 1] Close All Subwidgets
        (for _array_element (`/Game/Blueprints/UI/PauseMenu/BlockCollectorPauseMenuWidgetBR.WidgetList` _pausemenuwidget)
          (`Widget.RemoveFromParent` _array_element))
        (`Widget.RemoveFromParent` _pausemenuwidget)
        (`GameplayStatics.SetGamePaused` false)
        (`WidgetBlueprintLibrary.SetInputMode_GameOnly` _returnvalue)
        (set `PlayerController.bShowMouseCursor` false _returnvalue)))))

(event `EnhancedInput|/Game/Blueprints/Input/Driving/ChangeCameraBR`
  (params (ActionValue :type Boolean) (ElapsedSeconds :type "Float (double-precision)") (TriggeredSeconds :type "Float (double-precision)") (InputAction :type "InputAction Object Reference" :default "/Game/Blueprints/Input/Driving/ChangeCameraBR.ChangeCameraBR"))
  (:`Started`
    (`/Engine/EditorBlueprintResources/StandardMacros.FlipFlop`
      (:`A`
        ;[1 1 1] Change to 3rd Person cam
        (`ActorComponent.SetActive` (`self.Camera2ndPerson`) false false)
        (`ActorComponent.SetActive` (`self.Camera3rdPerson`) true false))
      (:`B`
        ;[1 1 1] Change to 2nd person Cam
        (`ActorComponent.SetActive` (`self.Camera3rdPerson`) false false)
        (`ActorComponent.SetActive` (`self.Camera2ndPerson`) true false)))))

(fn `UserConstructionScript`)
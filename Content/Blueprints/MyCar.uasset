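; MyCar is a car Blueprint that drives its skeletal mesh animation from the vehicle's current state.
; On BeginPlay it casts the mesh's anim instance to SK_Car1Temp_Skeleton_AnimBlueprint and caches it.
; Each Tick it copies current speed and steering angle into that instance, with debug prints along the way and no validity check on the cached reference.
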(event `self.ReceiveTick`
  (params (DeltaSeconds :type "Float (single-precision)"))
  (bind _animinstance (`self.AnimInstance`))
  (`KismetSystemLibrary.PrintString` "Event Tick")
  (bind _returnvalue (`self.GetCurrentSpeed`))
  (`KismetSystemLibrary.PrintString` (`KismetSystemLibrary.GetDisplayName` _animinstance))
  (set `/Game/Assets/Car/SK_Car1Temp_Skeleton_AnimBlueprint.Speed` _returnvalue _animinstance)
  (bind _returnvalue_2 (`self.GetCurrentSteeringAngle`))
  (set `/Game/Assets/Car/SK_Car1Temp_Skeleton_AnimBlueprint.Steering Angle` _returnvalue_2 _animinstance)
  (`KismetSystemLibrary.PrintString` (`KismetStringLibrary.Conv_DoubleToString` _returnvalue_2)))

(event `self.ReceiveBeginPlay`
  (bind _assk_car_1temp_skeleton_anim_blueprint (cast `/Game/Assets/Car/SK_Car1Temp_Skeleton_AnimBlueprint` (`SkeletalMeshComponent.GetAnimInstance` (`self.Mesh`)))
    (:`then`
      (`KismetSystemLibrary.PrintString` "AnimBlueprint Cast: Success")
      (set `self.AnimInstance` _assk_car_1temp_skeleton_anim_blueprint))
    (:`CastFailed`
      (`KismetSystemLibrary.PrintString` "AnimBlueprint Cast: Failed"))))

(fn `UserConstructionScript`)
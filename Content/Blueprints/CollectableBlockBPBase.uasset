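; Base Blueprint for a collectable block that awards points to a Car that overlaps it.
; On BeginPlay it copies Points into the block value, and Tick spins the Box at a frame-rate-independent rate.
; An overlapping actor that casts to Car receives the block value through AddPoints and the block destroys itself; other actors only trigger a "Failed" debug print.
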(event `self.ReceiveActorBeginOverlap`
  (params (OtherActor :type "Actor Object Reference"))
  (bind _ascar (cast `Car` OtherActor)
    (:`then`
      (bind _returnvalue (`self.GetBlockValue`))
      (`Car.AddPoints` _ascar _returnvalue)
      (`self.K2_DestroyActor`))
    (:`CastFailed`
      (`KismetSystemLibrary.PrintString` "Failed"))))

(event `self.ReceiveBeginPlay`
  (`self.SetBlockValue` (`self.Points`)))

(event `self.ReceiveTick`
  (params (DeltaSeconds :type "Float (single-precision)"))
  (`SceneComponent.K2_AddWorldRotation` (`self.Box`) (* (`self.Delta Rotation`) DeltaSeconds) false false))

(fn `UserConstructionScript`)